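; BOSSTURRET is an actor that drops a cylinder toward the PhysicsBallBP ball from high above, in a repeating cycle.
; For five seconds Tick makes the falling cylinder track the ball's X and Y, then locks them and moves Warning once to the ball's position.
; The fall uses hand-accumulated gravity applied per frame.
; Once locked and below the ball's height, it spawns a replacement high up and destroys itself.
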(event `self.ReceiveTick`
  (params (DeltaSeconds :type "Float (single-precision)"))
  (bind (_returnvalue_x _returnvalue_y _returnvalue_z) (`KismetMathLibrary.BreakVector` (`SceneComponent.K2_GetComponentLocation` (`self.Cylinder`))))
  (bind (_returnvalue_x_2 _returnvalue_y_2 _returnvalue_z_2) (`KismetMathLibrary.BreakVector` (`SceneComponent.K2_GetComponentLocation` (`self.Cylinder`))))
  (bind (_returnvalue_x_3 _returnvalue_y_3 _returnvalue_z_3) (`KismetMathLibrary.BreakVector` (`SceneComponent.K2_GetComponentLocation` (`self.Cylinder`))))
  (bind _output_get (set `self.delta` (+ DeltaSeconds (`self.delta`))))
  (if (> _output_get 5.0)
    (`|ExecutionSequence`
      (:`then_0`
        (`/Engine/EditorBlueprintResources/StandardMacros.DoOnce` false
          (:`Completed`
            (bind _outactors (`GameplayStatics.GetAllActorsOfClass` "/Game/RollingBP/Blueprints/PhysicsBallBP.PhysicsBallBP_C"))
            (bind _ball (`/Game/RollingBP/Blueprints/PhysicsBallBP.Ball` (`|GetArrayItem` _outactors)))
            (`SceneComponent.K2_SetWorldLocation` (`self.Warning`) (`SceneComponent.K2_GetComponentLocation` _ball) false false))))
      (:`then_1`
        (bind _output_get_2 (set `self.gravity` (- (`self.gravity`) (* 9.8 DeltaSeconds))))
        (`SceneComponent.K2_SetWorldLocation` (`self.Cylinder`) (`KismetMathLibrary.MakeVector` _returnvalue_x_3 _returnvalue_y_3 (+ _returnvalue_z_3 _output_get_2)) false false)
        (bind (_returnvalue_x_4 _returnvalue_y_4 _returnvalue_z_4) (`KismetMathLibrary.BreakVector` (`SceneComponent.K2_GetComponentLocation` _ball)))
        (if (< _returnvalue_z_2 _returnvalue_z_4)
          (`|SpawnActorFromClass` "BOSSTURRET_C" (`KismetMathLibrary.MakeTransform` (0.0 0.0 35000.0)) "Undefined" "OverrideRootScale" null null)
          (`self.K2_DestroyActor`))))
    (else
      (bind _outactors_2 (`GameplayStatics.GetAllActorsOfClass` "/Game/RollingBP/Blueprints/PhysicsBallBP.PhysicsBallBP_C"))
      (bind _output_get_3 (set `self.gravity` (- (`self.gravity`) (* 9.8 DeltaSeconds))))
      (bind (_returnvalue_x_5 _returnvalue_y_5) (`KismetMathLibrary.BreakVector` (`SceneComponent.K2_GetComponentLocation` (`/Game/RollingBP/Blueprints/PhysicsBallBP.Ball` (`|GetArrayItem` _outactors_2)))))
      (`SceneComponent.K2_SetWorldLocation` (`self.Cylinder`) (`KismetMathLibrary.MakeVector` _returnvalue_x_5 _returnvalue_y_5 (+ _returnvalue_z _output_get_3)) false false))))

(fn `UserConstructionScript`)