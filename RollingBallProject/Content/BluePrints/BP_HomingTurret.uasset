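; BP_HomingTurret is a turret that fires a projectile about once per second, using a Delay on Tick.
; When FollowingPlayer is set, it turns its base toward the PhysicsBallBP player and spawns a BP_Bullet aimed ahead of them.
; The lead point comes from player velocity times distance over a fixed divisor.
; Otherwise it leaves the base still and spawns a larger-scaled BP_BULLET2 along the spawn point's facing.
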(event `self.ReceiveBeginPlay`
  (bind _asphysics_ball_bp (cast `/Game/RollingBP/Blueprints/PhysicsBallBP` (`GameplayStatics.GetPlayerPawn` 0)))
  (set `self.Player` _asphysics_ball_bp))

(event `self.ReceiveTick`
  (params (DeltaSeconds :type "Float (single-precision)"))
  (bind _player (`self.Player`))
  (bind _returnvalue (`SceneComponent.K2_GetComponentLocation` (`self.SpawnPoint`)))
  (bind (_returnvalue_location _returnvalue_rotation) (`KismetMathLibrary.BreakTransform` (`SceneComponent.K2_GetComponentToWorld` (`self.SpawnPoint`))))
  (bind _returnvalue_2 (`SceneComponent.K2_GetComponentLocation` (`Actor.RootComponent` _player)))
  (if (`self.followingPlayer`)
    (`KismetSystemLibrary.Delay` 1.0)
    (`SceneComponent.K2_SetRelativeRotation` (`self.TurretBase`) (`KismetMathLibrary.FindLookAtRotation` _returnvalue _returnvalue_2) false false)
    (`|SpawnActorFromClass` "/Game/BluePrints/BP_Bullet.BP_Bullet_C" (`KismetMathLibrary.MakeTransform` (`SceneComponent.K2_GetComponentLocation` (`self.SpawnPoint`)) (`KismetMathLibrary.FindLookAtRotation` _returnvalue (+ _returnvalue_2 (* (`self.GetVelocity` _player) (/ (`self.GetDistanceTo` _player) 1200.0)))) (0.2 0.2 0.2)) "Undefined" "OverrideRootScale" null null)
    (else
      (`KismetSystemLibrary.Delay` 1.0)
      (`|SpawnActorFromClass` "/Game/BluePrints/BP_BULLET2.BP_BULLET2_C" (`KismetMathLibrary.MakeTransform` _returnvalue_location _returnvalue_rotation (2.0 2.0 2.0)) "Undefined" "OverrideRootScale" null null))))

(fn `UserConstructionScript`)