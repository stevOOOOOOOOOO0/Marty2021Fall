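; Gravity bomb actor that arms when a PhysicsBallBP enters its Collider, then pushes or pulls overlapping components.
; While armed, Tick applies Multiplier-scaled impulses along each tracked component's offset from the bomb and shrinks Arrow as a countdown.
; Time accumulates per component, so more components shorten the countdown.
; Past RunningTimer, it applies a reversed thousandfold impulse inside that loop and destroys itself.
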(event `self.Collider.OnComponentBeginOverlap`
  (params (OverlappedComponent :type "PrimitiveComponent Object Reference") (OtherActor :type "Actor Object Reference") (OtherComp :type "PrimitiveComponent Object Reference") (OtherBodyIndex :type Integer) (bFromSweep :type Boolean) (SweepResult :type "HitResult Structure (by ref)"))
  (cast `/Game/RollingBP/Blueprints/PhysicsBallBP` OtherActor
    (:`then`
      (set `self.Runner` true))
    (:`CastFailed`
      _))
  (`KismetArrayLibrary.Array_Add` (`self.Gravity Objects`) OtherComp))

(event `self.Collider.OnComponentEndOverlap`
  (params (OverlappedComponent :type "PrimitiveComponent Object Reference") (OtherActor :type "Actor Object Reference") (OtherComp :type "PrimitiveComponent Object Reference") (OtherBodyIndex :type Integer))
  (`KismetArrayLibrary.Array_RemoveItem` (`self.Gravity Objects`) OtherComp))

(event `self.ReceiveTick`
  (params (DeltaSeconds :type "Float (single-precision)"))
  ;[1 1 1] Runner Check
  (if (`self.Runner`)
    ;[1 1 1] Find Impulse Location and Apply it
    (for _array_element (`self.Gravity Objects`)
      (`PrimitiveComponent.AddImpulse` _array_element (* (- (`SceneComponent.K2_GetComponentLocation` _array_element) (`SceneComponent.K2_GetComponentLocation` (`self.BOMB`))) (`self.Multiplier`)) "None" false)
      ;[1 1 1] Add to the Timer and Decrease the Scale of Visual
      (bind _output_get (set `self.Time` (+ DeltaSeconds (`self.Time`))))
      (if (> _output_get (`self.RunningTimer`))
        ;[1 0 0] DESTROY
        (`PrimitiveComponent.AddImpulse` _array_element (* (- (`SceneComponent.K2_GetComponentLocation` _array_element) (`SceneComponent.K2_GetComponentLocation` (`self.BOMB`))) (* (`self.Multiplier`) -1000.0)) "None" false)
        (`self.K2_DestroyActor`)
        (else
          (`SceneComponent.SetRelativeScale3D` (`self.Arrow`) (`KismetMathLibrary.Conv_DoubleToVector` (/ (- (`self.RunningTimer`) _output_get) (`self.RunningTimer`)))))))))

(fn `UserConstructionScript`)