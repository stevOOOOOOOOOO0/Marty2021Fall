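; BP_BoostPickup is a respawning pickup that refills a car's boost meter on overlap.
; When a BP_Car enters the sphere, it adds BoostAmount to the car's Boost, capped at full.
; The pickup then hides its cylinder and disables collision, restoring both after a short delay.
; A BIGBOOST flag chooses between a full or partial refill amount at BeginPlay.
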(event `self.Sphere1.OnComponentBeginOverlap`
  (params (OverlappedComponent :type "PrimitiveComponent Object Reference") (OtherActor :type "Actor Object Reference") (OtherComp :type "PrimitiveComponent Object Reference") (OtherBodyIndex :type Integer) (bFromSweep :type Boolean) (SweepResult :type "HitResult Structure (by ref)"))
  (bind _asbp_car (cast `/Game/Blueprints/Car/BP_Car` OtherActor))
  (set `/Game/Blueprints/Car/BP_Car.Boost` (`KismetMathLibrary.FMin` (+ (`/Game/Blueprints/Car/BP_Car.Boost` _asbp_car) (`self.BoostAmount`)) 100.0) _asbp_car)
  (`SceneComponent.SetVisibility` (`self.Cylinder`) false true)
  (`PrimitiveComponent.SetCollisionEnabled` (`self.Sphere1`) "NoCollision")
  (`KismetSystemLibrary.Delay` 5.0)
  (`SceneComponent.SetVisibility` (`self.Cylinder`) true true)
  (`PrimitiveComponent.SetCollisionEnabled` (`self.Sphere1`) "QueryOnly"))

(event `self.ReceiveBeginPlay`
  (if (`self.BIGBOOST?`)
    (set `self.BoostAmount` 100.0)
    (else
      (set `self.BoostAmount` 25.0))))

(fn `UserConstructionScript`)